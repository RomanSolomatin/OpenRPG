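; Actor component that manages an RPG character's stats, stat points, HP/SP bars and their UI widgets, with save-slot persistence.
; Equipment and point spending change base values, and Max HP/SP changes also resize the matching bars.
; Per-bar looping timers drive regeneration and pause at full value.
; Timed buffs and nerfs accumulate in a separate amount per stat, reverted by a one-second timer that pauses when none remain.
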(fn `AddStatPoints`
  (params (Amount :type Integer))
  (bind _returnvalue (+ (`self.StatPoints`) Amount))
  (set `self.StatPoints` (`KismetMathLibrary.Clamp` _returnvalue 0 _returnvalue))
  (`self.UpdateStatsWidget`)
  (return))

(fn `AddStatValue`
  (params (Stat :type "/Game/OpenRPG/StatsSystem/Enums/e_Stat Enum" :default "NewEnumerator0") (Amount :type Integer) (`ConsumesPoints?` :type Boolean))
  (locals (LocalStat :type "/Game/OpenRPG/StatsSystem/Enums/e_Stat Enum" :default "NewEnumerator0") (LocalAmount :type Integer) (LocalConsumes :type Boolean))
  (bind _localamount (`local.LocalAmount`))
  (set `local.LocalStat` Stat)
  (set `local.LocalAmount` Amount)
  (set `local.LocalConsumes` `ConsumesPoints?`)
  (bind (_index _foundstat) (`self.GetStat` (`local.LocalStat`)))
  (bind (_stat _value _buffnerfamount _ispercentage_) (break `/Game/OpenRPG/StatsSystem/Structs/s_Stat` _foundstat))
  (`KismetArrayLibrary.Array_Set` (`self.Stats`) _index (make `/Game/OpenRPG/StatsSystem/Structs/s_Stat` _stat (+ (`local.LocalAmount`) _value) _buffnerfamount _ispercentage_))
  (if (`local.LocalConsumes`)
    (set `self.StatPoints` (- (`self.StatPoints`) (`local.LocalAmount`))))
  (switch `/Game/OpenRPG/StatsSystem/Enums/e_Stat` (`local.LocalStat`)
    (:`NewEnumerator0`
      (`self.OnMaxHPUpdated` _localamount))
    (:`NewEnumerator1`
      (`self.OnMaxSPUpdated` _localamount))
    (:`NewEnumerator2`
      _)
    (:`NewEnumerator3`
      _)
    (:`NewEnumerator4`
      _)
    (:`NewEnumerator5`
      _)
    (:`NewEnumerator6`
      _)
    (:`NewEnumerator7`
      _)
    (:`NewEnumerator8`
      _)
    (:`NewEnumerator9`
      _))
  (`self.UpdateStatsWidget`)
  (return))

(fn `BuffStat`
  (params (Stat :type "/Game/OpenRPG/StatsSystem/Enums/e_Stat Enum" :default "NewEnumerator0") (Amount :type Integer) (Duration :type Integer))
  (locals (LocalStat :type "/Game/OpenRPG/StatsSystem/Enums/e_Stat Enum" :default "NewEnumerator0") (LocalAmount :type Integer) (LocalDuration :type Integer))
  (set `local.LocalStat` Stat)
  (set `local.LocalAmount` Amount)
  (set `local.LocalDuration` Duration)
  (`KismetArrayLibrary.Array_Add` (`self.Modifiers`) (make `/Game/OpenRPG/StatsSystem/Structs/s_Modifier` (`local.LocalStat`) (`local.LocalAmount`) (+ (`KismetMathLibrary.Now`) (`KismetMathLibrary.MakeTimespan` 0 0 0 (`local.LocalDuration`)))))
  (bind (_index _foundstat) (`self.GetStat` (`local.LocalStat`)))
  (bind (_stat _value _buffnerfamount _ispercentage_) (break `/Game/OpenRPG/StatsSystem/Structs/s_Stat` _foundstat))
  (`KismetArrayLibrary.Array_Set` (`self.Stats`) _index (make `/Game/OpenRPG/StatsSystem/Structs/s_Stat` _stat _value (+ _buffnerfamount (`local.LocalAmount`)) _ispercentage_))
  (`self.UpdateStatsWidget`)
  (if (`KismetSystemLibrary.K2_IsTimerPausedHandle` (`self.ModifiersTimer`))
    (`KismetSystemLibrary.K2_UnPauseTimerHandle` (`self.ModifiersTimer`))
    (return)
    (else
      (return))))

(fn `GetBarData`
  (params (BarStat :type "/Game/OpenRPG/StatsSystem/Enums/e_BarStat Enum" :default "NewEnumerator0"))
  (returns (Data :type "/Game/OpenRPG/StatsSystem/Structs/s_BarStat Structure"))
  (locals (LocalBarStat :type "/Game/OpenRPG/StatsSystem/Enums/e_BarStat Enum" :default "NewEnumerator0") (LocalData :type "/Game/OpenRPG/StatsSystem/Structs/s_BarStat Structure"))
  (set `local.LocalBarStat` BarStat)
  (for _array_element (`self.BarStats`)
    (if (`|EnumEquality` (`.BarStat_21_244CAB4941E4201DC3B2F984AF8666EF` (break `/Game/OpenRPG/StatsSystem/Structs/s_BarStat` _array_element)) (`local.LocalBarStat`))
      (set `local.LocalData` _array_element)
      (break)))
  (return (`local.LocalData`)))

(fn `GetBarWidget`
  (params (BarStat :type "/Game/OpenRPG/StatsSystem/Enums/e_BarStat Enum" :default "NewEnumerator0"))
  (returns (Widget :type "/Game/OpenRPG/StatsSystem/Widgets/WB_StatBar Object Reference"))
  (locals (LocalBarStat :type "/Game/OpenRPG/StatsSystem/Enums/e_BarStat Enum" :default "NewEnumerator0") (LocalWidget :type "/Game/OpenRPG/StatsSystem/Widgets/WB_StatBar Object Reference"))
  (set `local.LocalBarStat` BarStat)
  (for _array_element (`self.BarWidgets`)
    (if (`|EnumEquality` (`/Game/OpenRPG/StatsSystem/Widgets/WB_StatBar.BarStat` _array_element) (`local.LocalBarStat`))
      (set `local.LocalWidget` _array_element)
      (break)))
  (return (`local.LocalWidget`)))

(fn `GetCurrentLvl`
  (returns (Lvl :type Integer))
  (return (`self.CurrentLvl`)))

(fn `GetStat`
  (params (Stat :type "/Game/OpenRPG/StatsSystem/Enums/e_Stat Enum" :default "NewEnumerator0"))
  (returns (Index :type Integer) (FoundStat :type "/Game/OpenRPG/StatsSystem/Structs/s_Stat Structure"))
  (locals (LocalStat :type "/Game/OpenRPG/StatsSystem/Enums/e_Stat Enum" :default "NewEnumerator0") (LocalIndex :type Integer :default -1) (LocalStatFound :type "/Game/OpenRPG/StatsSystem/Structs/s_Stat Structure"))
  (set `local.LocalStat` Stat)
  (for (_array_element _array_index) (`self.Stats`)
    (if (`|EnumEquality` (`.Stat_5_AC4A4C4E4D93310998F3B6871A55322A` (break `/Game/OpenRPG/StatsSystem/Structs/s_Stat` _array_element)) (`local.LocalStat`))
      (set `local.LocalIndex` _array_index)
      (set `local.LocalStatFound` _array_element)
      (break)))
  (return (`local.LocalIndex`) (`local.LocalStatFound`)))

(fn `GetStatData`
  (params (Stat :type "/Game/OpenRPG/StatsSystem/Enums/e_Stat Enum" :default "NewEnumerator0"))
  (returns (Value :type Integer) (`Buff/Nerf Amount` :type Integer) (`IsPercentage?` :type Boolean))
  (locals (LocalStat :type "/Game/OpenRPG/StatsSystem/Enums/e_Stat Enum" :default "NewEnumerator0"))
  (bind _output_get (set `local.LocalStat` Stat))
  (bind (_index _foundstat) (`self.GetStat` _output_get))
  (bind ((`Value_7_17529A2749D35F51CCAB84A767D1919A` _value) (`BuffNerfAmount_11_59A489084333A86CBDA7879082D9BFA7` _buffnerfamount) (`IsPercentage?_8_0778F836481175FF0FEDBABC501782DB` _ispercentage_)) (break `/Game/OpenRPG/StatsSystem/Structs/s_Stat` _foundstat))
  (return _value _buffnerfamount _ispercentage_))

(fn `GetStatPoints`
  (returns (StatPoints :type Integer))
  (return (`self.StatPoints`)))

(fn `HandleRegenerationTimers`
  (params (BarStat :type "/Game/OpenRPG/StatsSystem/Enums/e_BarStat Enum" :default "NewEnumerator0"))
  (locals (LocalData :type "/Game/OpenRPG/StatsSystem/Structs/s_BarStat Structure") (LocalTimer :type "TimerHandle Structure"))
  (bind ((`MaxValue_7_EFFDE6874913F29171ED169ABFC904D0` _maxvalue) (`CurrentValue_22_430DCD794A2E2F05FDEAF3881E7CE7DF` _currentvalue) (`TimerIndex_24_B60BA1EB46174C8A8A35FD8ACCAF8820` _timerindex)) (break `/Game/OpenRPG/StatsSystem/Structs/s_BarStat` (`local.LocalData`)))
  (bind ((`MaxValue_7_EFFDE6874913F29171ED169ABFC904D0` _maxvalue_2) (`CurrentValue_22_430DCD794A2E2F05FDEAF3881E7CE7DF` _currentvalue_2)) (break `/Game/OpenRPG/StatsSystem/Structs/s_BarStat` (`local.LocalData`)))
  (set `local.LocalData` (`self.GetBarData` BarStat))
  (bind _output_get (set `local.LocalTimer` (`|GetArrayItem` (`self.Timers`) _timerindex)))
  (if (and (`KismetSystemLibrary.K2_IsTimerPausedHandle` _output_get) (!= _maxvalue _currentvalue))
    (`KismetSystemLibrary.K2_UnPauseTimerHandle` (`local.LocalTimer`))
    (return)
    (elif (and (not (`KismetSystemLibrary.K2_IsTimerPausedHandle` (`local.LocalTimer`))) (== _maxvalue_2 _currentvalue_2))
      (`KismetSystemLibrary.K2_PauseTimerHandle` (`local.LocalTimer`))
      (return)
      (else
        (return)))))

(fn `HPRegenerationTick`
  (bind ((`MaxValue_7_EFFDE6874913F29171ED169ABFC904D0` _maxvalue) (`RegenPercent_28_5FDDC65748DC380C629AFEB811A27381` _regenpercent)) (break `/Game/OpenRPG/StatsSystem/Structs/s_BarStat` (`self.GetBarData` "NewEnumerator0")))
  (`self.ModifyBarStat` "NewEnumerator0" (`KismetMathLibrary.FTrunc` (/ (* (`KismetMathLibrary.Conv_IntToDouble` _maxvalue) _regenpercent) 100.0)))
  (return))

(fn `Initialize`
  (params (WB_Stat :type "/Game/OpenRPG/StatsSystem/Widgets/WB_StatsList Object Reference") (WB_Bars :type "Array of /Game/OpenRPG/StatsSystem/Widgets/WB_StatBar Object Reference"))
  (set `self.StatsWidget` WB_Stat)
  (set `self.BarWidgets` WB_Bars)
  (bind _asbp_custom_player_controller (cast `/Game/OpenRPG/Shared/Blueprints/BP_CustomPlayerController` (`self.GetOwner`)))
  (set `self.PlayerController` _asbp_custom_player_controller)
  (`self.LoadStats`)
  (`self.SetupRegeneration`)
  (bind _returnvalue (`KismetSystemLibrary.K2_SetTimer` null "ModifiersHandler" 1.0 true))
  (set `self.ModifiersTimer` _returnvalue)
  (bind _enumvalue (foreach `/Game/OpenRPG/StatsSystem/Enums/e_Stat`) ; Just temp
    (:`LoopBody`
      (bind (_index _foundstat) (`self.GetStat` _enumvalue))
      (bind (_stat _value _buffnerfamount _ispercentage_) (break `/Game/OpenRPG/StatsSystem/Structs/s_Stat` _foundstat))
      (`KismetArrayLibrary.Array_Set` (`self.Stats`) _index (make `/Game/OpenRPG/StatsSystem/Structs/s_Stat` _stat _value 0 _ispercentage_)))
    (:`then`
      (for _array_element (`self.BarWidgets`)
        (`self.UpdateBarStat` (`/Game/OpenRPG/StatsSystem/Widgets/WB_StatBar.BarStat` _array_element)))
      (`/Game/OpenRPG/StatsSystem/Widgets/WB_StatsList.Initialize` (`self.StatsWidget`) self)
      (return))))

(fn `IsBuffered?`
  (params (Stat :type "/Game/OpenRPG/StatsSystem/Enums/e_Stat Enum" :default "NewEnumerator0"))
  (returns (`Buff?` :type Boolean))
  (return (> (`.Buff/Nerf Amount` (`self.GetStatData` Stat)) 0)))

(fn `IsNerfed?`
  (params (Stat :type "/Game/OpenRPG/StatsSystem/Enums/e_Stat Enum" :default "NewEnumerator0"))
  (returns (`Nerf?` :type Boolean))
  (return (< (`.Buff/Nerf Amount` (`self.GetStatData` Stat)) 0)))

(fn `LoadStats`
  (bind _statssaveobject (`self.StatsSaveObject`))
  (bind _returnvalue (`GameplayStatics.DoesSaveGameExist` (`self.SaveSlotName`)))
  (if _returnvalue
    (`/Engine/EditorBlueprintResources/StandardMacros.IsValid` (`self.StatsSaveObject`)
      (:`Is Valid`
        _)
      (:`Is Not Valid`
        (bind _returnvalue_2 (`GameplayStatics.LoadGameFromSlot` (`self.SaveSlotName`)))
        (bind _asstats_save (cast `/Game/OpenRPG/StatsSystem/Blueprints/StatsSave` _returnvalue_2)
          (:`then`
            (set `self.StatsSaveObject` _asstats_save))
          (:`CastFailed`
            (return)))))
    (set `self.Stats` (`/Game/OpenRPG/StatsSystem/Blueprints/StatsSave.SavedStats` (`self.StatsSaveObject`)))
    (set `self.BarStats` (`/Game/OpenRPG/StatsSystem/Blueprints/StatsSave.SavedBarStats` (`self.StatsSaveObject`)))
    (set `self.CurrentLvl` (`/Game/OpenRPG/StatsSystem/Blueprints/StatsSave.SavedLvl` _statssaveobject))
    (set `self.StatPoints` (`/Game/OpenRPG/StatsSystem/Blueprints/StatsSave.SavedStatPoints` _statssaveobject))
    (return)
    (else
      ;[1 1 1] Load datatable maybe?
      (return))))

(fn `ModifiersHandler`
  (if (> (`KismetArrayLibrary.Array_Length` (`self.Modifiers`)) 0)
    (for (_array_element _array_index) (`self.Modifiers`)
      (bind (_stat _amount _endtime) (break `/Game/OpenRPG/StatsSystem/Structs/s_Modifier` _array_element))
      (if (<= _endtime (`KismetMathLibrary.Now`))
        (bind (_index _foundstat) (`self.GetStat` _stat))
        (bind (_stat_2 _value _buffnerfamount _ispercentage_) (break `/Game/OpenRPG/StatsSystem/Structs/s_Stat` _foundstat))
        (`KismetArrayLibrary.Array_Set` (`self.Stats`) _index (make `/Game/OpenRPG/StatsSystem/Structs/s_Stat` _stat_2 _value (+ _buffnerfamount (* _amount -1)) _ispercentage_))
        (`KismetArrayLibrary.Array_Remove` (`self.Modifiers`) _array_index)))
    (`self.UpdateStatsWidget`)
    (return)
    (else
      (`KismetSystemLibrary.K2_PauseTimerHandle` (`self.ModifiersTimer`))
      (return))))

(fn `ModifyBarStat`
  (params (BarStat :type "/Game/OpenRPG/StatsSystem/Enums/e_BarStat Enum" :default "NewEnumerator0") (By :type Integer) (`Animated?` :type Boolean))
  (locals (LocalBarStat :type "/Game/OpenRPG/StatsSystem/Enums/e_BarStat Enum" :default "NewEnumerator0") (LocalBy :type Integer) (LocalAnimated :type Boolean) (LocalBarData :type "/Game/OpenRPG/StatsSystem/Structs/s_BarStat Structure"))
  (set `local.LocalBarStat` BarStat)
  (set `local.LocalBy` By)
  (set `local.LocalAnimated` `Animated?`)
  (if (!= (`local.LocalBy`) 0)
    (if (`local.LocalAnimated`)
      (return)
      (else
        (bind _output_get (set `local.LocalBarData` (`self.GetBarData` (`local.LocalBarStat`))))
        (bind ((`MaxValue_7_EFFDE6874913F29171ED169ABFC904D0` _maxvalue) (`CurrentValue_22_430DCD794A2E2F05FDEAF3881E7CE7DF` _currentvalue)) (break `/Game/OpenRPG/StatsSystem/Structs/s_BarStat` _output_get))
        (bind _structout (setmembers `/Game/OpenRPG/StatsSystem/Structs/s_BarStat` :`StructRef` (`local.LocalBarData`) :`CurrentValue` (`KismetMathLibrary.Clamp` (+ _currentvalue (`local.LocalBy`)) 0 _maxvalue)))
        (`self.SetBarData` (`local.LocalBarStat`) _structout)
        (`self.HandleRegenerationTimers` (`local.LocalBarStat`))
        (`self.UpdateBarStat` (`local.LocalBarStat`))
        (return)))
    (else
      (return))))

(fn `NerfStat`
  (params (Stat :type "/Game/OpenRPG/StatsSystem/Enums/e_Stat Enum" :default "NewEnumerator0") (Amount :type Integer) (Duration :type Integer))
  (locals (LocalStat :type "/Game/OpenRPG/StatsSystem/Enums/e_Stat Enum") (LocalAmount :type Integer) (LocalDuration :type Integer))
  (set `local.LocalStat` Stat)
  (set `local.LocalAmount` Amount)
  (set `local.LocalDuration` Duration)
  (`KismetArrayLibrary.Array_Add` (`self.Modifiers`) (make `/Game/OpenRPG/StatsSystem/Structs/s_Modifier` (`local.LocalStat`) (* (`local.LocalAmount`) -1) (+ (`KismetMathLibrary.Now`) (`KismetMathLibrary.MakeTimespan` 0 0 0 (`local.LocalDuration`)))))
  (bind (_index _foundstat) (`self.GetStat` (`local.LocalStat`)))
  (bind (_stat _value _buffnerfamount _ispercentage_) (break `/Game/OpenRPG/StatsSystem/Structs/s_Stat` _foundstat))
  (`KismetArrayLibrary.Array_Set` (`self.Stats`) _index (make `/Game/OpenRPG/StatsSystem/Structs/s_Stat` _stat _value (- _buffnerfamount (`local.LocalAmount`)) _ispercentage_))
  (`self.UpdateStatsWidget`)
  (if (`KismetSystemLibrary.K2_IsTimerPausedHandle` (`self.ModifiersTimer`))
    (`KismetSystemLibrary.K2_UnPauseTimerHandle` (`self.ModifiersTimer`))
    (return)
    (else
      (return))))

(fn `OnMaxHPUpdated`
  (params (Amount :type Integer))
  (locals (LocalAmount :type Integer) (LocalData :type "/Game/OpenRPG/StatsSystem/Structs/s_BarStat Structure"))
  (set `local.LocalAmount` Amount)
  (bind _output_get (set `local.LocalData` (`self.GetBarData` "NewEnumerator0")))
  (bind ((`MaxValue_7_EFFDE6874913F29171ED169ABFC904D0` _maxvalue) (`CurrentValue_22_430DCD794A2E2F05FDEAF3881E7CE7DF` _currentvalue)) (break `/Game/OpenRPG/StatsSystem/Structs/s_BarStat` _output_get))
  (bind _returnvalue (+ _maxvalue (`local.LocalAmount`)))
  (bind _structout (setmembers `/Game/OpenRPG/StatsSystem/Structs/s_BarStat` :`StructRef` _output_get :`MaxValue` _returnvalue :`CurrentValue` (`KismetMathLibrary.Clamp` _currentvalue 0 _returnvalue)))
  (`self.SetBarData` "NewEnumerator0" _structout)
  (`self.HandleRegenerationTimers` "NewEnumerator0")
  (`self.UpdateBarStat` "NewEnumerator0")
  (return))

(fn `OnMaxSPUpdated`
  (params (Amount :type Integer))
  (locals (LocalAmount :type Integer) (LocalData :type "/Game/OpenRPG/StatsSystem/Structs/s_BarStat Structure"))
  (set `local.LocalAmount` Amount)
  (bind _output_get (set `local.LocalData` (`self.GetBarData` "NewEnumerator1")))
  (bind ((`MaxValue_7_EFFDE6874913F29171ED169ABFC904D0` _maxvalue) (`CurrentValue_22_430DCD794A2E2F05FDEAF3881E7CE7DF` _currentvalue)) (break `/Game/OpenRPG/StatsSystem/Structs/s_BarStat` _output_get))
  (bind _returnvalue (+ _maxvalue (`local.LocalAmount`)))
  (bind _structout (setmembers `/Game/OpenRPG/StatsSystem/Structs/s_BarStat` :`StructRef` _output_get :`MaxValue` _returnvalue :`CurrentValue` (`KismetMathLibrary.Clamp` _currentvalue 0 _returnvalue)))
  (`self.SetBarData` "NewEnumerator1" _structout)
  (`self.HandleRegenerationTimers` "NewEnumerator1")
  (`self.UpdateBarStat` "NewEnumerator1")
  (return))

(fn `RestartRegeneration`
  (params (BarStat :type "/Game/OpenRPG/StatsSystem/Enums/e_BarStat Enum" :default "NewEnumerator0"))
  (locals (LocalTimer :type "TimerHandle Structure"))
  (bind ((`HasRegeneration?_12_4F51CF9A42E240CB3CC8AE9D47A4DDEB` _hasregeneration_) (`TimerIndex_24_B60BA1EB46174C8A8A35FD8ACCAF8820` _timerindex)) (break `/Game/OpenRPG/StatsSystem/Structs/s_BarStat` (`self.GetBarData` BarStat)))
  (if _hasregeneration_
    (bind _output_get (set `local.LocalTimer` (`|GetArrayItem` (`self.Timers`) _timerindex)))
    (if (`KismetSystemLibrary.K2_IsTimerPausedHandle` _output_get)
      (`KismetSystemLibrary.K2_PauseTimerHandle` (`local.LocalTimer`))
      (return)
      (else
        (return)))
    (else
      (return))))

(fn `SaveStats`
  (`/Engine/EditorBlueprintResources/StandardMacros.IsValid` (`self.StatsSaveObject`)
    (:`Is Valid`
      _)
    (:`Is Not Valid`
      (bind _returnvalue (`GameplayStatics.CreateSaveGameObject` "/Game/OpenRPG/StatsSystem/Blueprints/StatsSave.StatsSave_C"))
      (set `self.StatsSaveObject` _returnvalue)))
  (set `/Game/OpenRPG/StatsSystem/Blueprints/StatsSave.SavedStats` (`self.Stats`) (`self.StatsSaveObject`))
  (set `/Game/OpenRPG/StatsSystem/Blueprints/StatsSave.SavedBarStats` (`self.BarStats`) (`self.StatsSaveObject`))
  (set `/Game/OpenRPG/StatsSystem/Blueprints/StatsSave.SavedStatPoints` (`self.StatPoints`) (`self.StatsSaveObject`))
  (set `/Game/OpenRPG/StatsSystem/Blueprints/StatsSave.SavedLvl` (`self.CurrentLvl`) (`self.StatsSaveObject`))
  (`GameplayStatics.SaveGameToSlot` (`self.StatsSaveObject`) (`self.SaveSlotName`))
  (return))

(fn `SetBarData`
  (params (BarStat :type "/Game/OpenRPG/StatsSystem/Enums/e_BarStat Enum" :default "NewEnumerator0") (NewData :type "/Game/OpenRPG/StatsSystem/Structs/s_BarStat Structure"))
  (locals (LocalBarStat :type "/Game/OpenRPG/StatsSystem/Enums/e_BarStat Enum") (LocalNewData :type "/Game/OpenRPG/StatsSystem/Structs/s_BarStat Structure"))
  (set `local.LocalBarStat` BarStat)
  (set `local.LocalNewData` NewData)
  (for (_array_element _array_index) (`self.BarStats`)
    (if (`|EnumEquality` (`.BarStat_21_244CAB4941E4201DC3B2F984AF8666EF` (break `/Game/OpenRPG/StatsSystem/Structs/s_BarStat` _array_element)) (`local.LocalBarStat`))
      (`KismetArrayLibrary.Array_Set` (`self.BarStats`) _array_index (`local.LocalNewData`))
      (break)))
  (return))

(fn `SetupRegeneration`
  (locals (LocalStat :type "/Game/OpenRPG/StatsSystem/Enums/e_BarStat Enum"))
  (for (_array_element _array_index) (`self.BarStats`)
    (bind ((`BarStat_21_244CAB4941E4201DC3B2F984AF8666EF` _barstat) (`HasRegeneration?_12_4F51CF9A42E240CB3CC8AE9D47A4DDEB` _hasregeneration_) (`RegenerationTick_18_BBA1597545CCA1D293B9329281E3E9B8` _regenerationtick) (`RegFuncName_29_C1C626F74B3168810AE763BEEEA19977` _regfuncname)) (break `/Game/OpenRPG/StatsSystem/Structs/s_BarStat` _array_element))
    (set `local.LocalStat` _barstat)
    (if _hasregeneration_
      (bind _returnvalue (`KismetSystemLibrary.K2_SetTimer` null (`KismetStringLibrary.Conv_NameToString` _regfuncname) _regenerationtick true))
      (bind _returnvalue_2 (`KismetArrayLibrary.Array_Add` (`self.Timers`) _returnvalue))
      (bind _structout (setmembers `/Game/OpenRPG/StatsSystem/Structs/s_BarStat` :`StructRef` _array_element :`TimerIndex` _returnvalue_2))
      (`KismetArrayLibrary.Array_Set` (`self.BarStats`) _array_index _structout)
      (`self.HandleRegenerationTimers` (`local.LocalStat`))))
  (return))

(fn `SPRegenerationTick`
  (bind ((`MaxValue_7_EFFDE6874913F29171ED169ABFC904D0` _maxvalue) (`RegenPercent_28_5FDDC65748DC380C629AFEB811A27381` _regenpercent)) (break `/Game/OpenRPG/StatsSystem/Structs/s_BarStat` (`self.GetBarData` "NewEnumerator1")))
  (`self.ModifyBarStat` "NewEnumerator1" (`KismetMathLibrary.FTrunc` (/ (* (`KismetMathLibrary.Conv_IntToDouble` _maxvalue) _regenpercent) 100.0)))
  (return))

(fn `StopRegeneration`
  (params (BarStat :type "/Game/OpenRPG/StatsSystem/Enums/e_BarStat Enum" :default "NewEnumerator0"))
  (locals (LocalTimer :type "TimerHandle Structure"))
  (bind ((`HasRegeneration?_12_4F51CF9A42E240CB3CC8AE9D47A4DDEB` _hasregeneration_) (`TimerIndex_24_B60BA1EB46174C8A8A35FD8ACCAF8820` _timerindex)) (break `/Game/OpenRPG/StatsSystem/Structs/s_BarStat` (`self.GetBarData` BarStat)))
  (if _hasregeneration_
    (bind _output_get (set `local.LocalTimer` (`|GetArrayItem` (`self.Timers`) _timerindex)))
    (if (`KismetSystemLibrary.K2_IsTimerPausedHandle` _output_get)
      (return)
      (else
        (`KismetSystemLibrary.K2_UnPauseTimerHandle` (`local.LocalTimer`))
        (return)))
    (else
      (return))))

(fn `ToggleStatsVisibility`
  (bind _returnvalue (select `bool` (`Widget.IsVisible` (`self.StatsWidget`)) :`false` "Visible" :`true` "Hidden" :!type "ESlateVisibility Enum"))
  (`Widget.SetVisibility` (`self.StatsWidget`) _returnvalue)
  (`Widget.SetIsEnabled` (`self.StatsWidget`) (select `ESlateVisibility` _returnvalue :`Hidden` true))
  (return))

(fn `UpdateBarStat`
  (params (BarStat :type "/Game/OpenRPG/StatsSystem/Enums/e_BarStat Enum" :default "NewEnumerator0"))
  (locals (LocalBarWidget :type "/Game/OpenRPG/StatsSystem/Widgets/WB_StatBar Object Reference") (LocalBarStat :type "/Game/OpenRPG/StatsSystem/Enums/e_BarStat Enum" :default "NewEnumerator0") (LocalBarData :type "/Game/OpenRPG/StatsSystem/Structs/s_BarStat Structure"))
  (bind _localbarwidget (`local.LocalBarWidget`))
  (bind ((`MaxValue_7_EFFDE6874913F29171ED169ABFC904D0` _maxvalue) (`CurrentValue_22_430DCD794A2E2F05FDEAF3881E7CE7DF` _currentvalue)) (break `/Game/OpenRPG/StatsSystem/Structs/s_BarStat` (`local.LocalBarData`)))
  (bind ((`MaxValue_7_EFFDE6874913F29171ED169ABFC904D0` _maxvalue_2) (`CurrentValue_22_430DCD794A2E2F05FDEAF3881E7CE7DF` _currentvalue_2)) (break `/Game/OpenRPG/StatsSystem/Structs/s_BarStat` (`local.LocalBarData`)))
  (bind _returnvalue (`KismetMathLibrary.FClamp` (/ (`KismetMathLibrary.Conv_IntToDouble` _currentvalue) (`KismetMathLibrary.Conv_IntToDouble` _maxvalue))))
  (set `local.LocalBarStat` BarStat)
  (bind _output_get (set `local.LocalBarWidget` (`self.GetBarWidget` BarStat)))
  (`/Engine/EditorBlueprintResources/StandardMacros.IsValid` _output_get
    (:`Is Valid`
      (set `local.LocalBarData` (`self.GetBarData` (`local.LocalBarStat`)))
      (`ProgressBar.SetPercent` (`/Game/OpenRPG/StatsSystem/Widgets/WB_StatBar.StatProgressBar` (`local.LocalBarWidget`)) _returnvalue)
      (if (`/Game/OpenRPG/StatsSystem/Widgets/WB_StatBar.ShowsFloatTextValues?` _localbarwidget)
        (`TextBlock.SetText` (`/Game/OpenRPG/StatsSystem/Widgets/WB_StatBar.ValuesText` (`local.LocalBarWidget`)) (select `bool` (`/Game/OpenRPG/StatsSystem/Widgets/WB_StatBar.ShowsPercentage?` _localbarwidget) :`false` (`|FormatText` "{CurrentValue}/{MaxValue}" _currentvalue_2 _maxvalue_2) :`true` (`|FormatText` "{Percentage}%" (* _returnvalue 100.0))))
        (return)
        (else
          (return))))
    (:`Is Not Valid`
      (return))))

(fn `UpdateStatsFromEquipment`
  (params (NewEquipmentStats :type "Array of /Game/OpenRPG/EquipmentSystem/Structs/s_EquipmentStat Structure") (`Equip?` :type Boolean))
  (locals (LocalNewStats :type "Array of /Game/OpenRPG/EquipmentSystem/Structs/s_EquipmentStat Structure") (`LocalEquip?` :type Boolean))
  (set `local.LocalNewStats` NewEquipmentStats)
  (set `local.LocalEquip?` `Equip?`)
  (for _array_element (`local.LocalNewStats`)
    (bind (_stat _value) (break `/Game/OpenRPG/EquipmentSystem/Structs/s_EquipmentStat` _array_element))
    (`self.AddStatValue` _stat (`KismetMathLibrary.SelectInt` _value (* _value -1) (`local.LocalEquip?`))))
  (return))

(fn `UpdateStatsWidget`
  (`PanelWidget.ClearChildren` (`/Game/OpenRPG/StatsSystem/Widgets/WB_StatsList.StatsEntryList` (`self.StatsWidget`)))
  (for _array_element (`self.Stats`)
    (bind _returnvalue (`|CreateWidget` "/Game/OpenRPG/StatsSystem/Widgets/WB_StatEntry.WB_StatEntry_C" null _array_element (> (`self.StatPoints`) 0)))
    (`PanelWidget.AddChild` (`/Game/OpenRPG/StatsSystem/Widgets/WB_StatsList.StatsEntryList` (`self.StatsWidget`)) _returnvalue))
  (`TextBlock.SetText` (`/Game/OpenRPG/StatsSystem/Widgets/WB_StatsList.StatPointsText` (`self.StatsWidget`)) (`|FormatText` "Stat points: {Points}" (`self.StatPoints`)))
  (return))