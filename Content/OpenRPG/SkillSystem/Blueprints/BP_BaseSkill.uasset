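; Base skill Blueprint for an RPG skill system, handling a spell's cast from validation through cooldown.
; On BeginPlay it loads its info and current stage from DT_Skills by ID.
; Casting checks cooldown, spends mana, notifies SkillComponent, then either plays a montage rate-scaled by casting time with movement disabled or simply delays.
; Completion starts a cooldown timeline that drives the hotkey's radial material, countdown text and enabled state.
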(event `UpdateStageInfo`
  (bind _returnvalue (`|GetDataTableRow` "/Game/OpenRPG/SkillSystem/DataTables/DT_Skills.DT_Skills" (`KismetStringLibrary.Conv_StringToName` (`KismetStringLibrary.Conv_IntToString` (`self.ID`))))
    (:`then`
      (bind (_class _name _icon _description _target _animation _stages) (break `/Game/OpenRPG/SkillSystem/DataTables/s_SkillData` _returnvalue))
      (set `self.Info` (make `/Game/OpenRPG/SkillSystem/Structs/s_SkillInfo` _class _name _icon _description _target _animation (`|GetArrayItem` _stages (`self.CurrentStageIndex`)))))))

(event `self.ReceiveBeginPlay`
  (`self.UpdateStageInfo`))

(event `TrySpellCast`
  ;[0.007734 0.5562 1] 1. Conditions needed to cast the spell
  (if (not (`self.OnCooldown?`))
    (`self.ManaCheck`)))

(event `SkillNotify`)

(event `ManaCheck`
  (bind ((`ManaCost_12_4D22187649CEFAF6C0367EA57C4DD532` _manacost)) (break `/Game/OpenRPG/SkillSystem/Structs/s_SkillStage` (`.Stage_18_B74872704392C835D0B405866CA6B20E` (break `/Game/OpenRPG/SkillSystem/Structs/s_SkillInfo` (`self.Info`)))))
  ;[0.1797 0.4482 1] 2. Check for enough mana
  (if (>= (`/Game/OpenRPG/StatsSystem/Blueprints/BPC_StatsHandler.GetCurrentBarValue` (`/Game/OpenRPG/Shared/Blueprints/BP_CustomPlayerController.BPC_StatsHandler` (`/Game/OpenRPG/SkillSystem/Blueprints/BPC_SkillsHandler.PlayerControllerOwner` (`self.SkillComponent`))) "NewEnumerator1") _manacost)
    (`/Game/OpenRPG/StatsSystem/Blueprints/BPC_StatsHandler.ModifyBarStat` (`/Game/OpenRPG/Shared/Blueprints/BP_CustomPlayerController.BPC_StatsHandler` (`/Game/OpenRPG/SkillSystem/Blueprints/BPC_SkillsHandler.PlayerControllerOwner` (`self.SkillComponent`))) "NewEnumerator1" (* _manacost -1.0))
    (`self.InitializeCasting`)
    (else
      (`KismetSystemLibrary.PrintString` "Not enough mana"))))

(event `InitializeCasting`
  (bind _hotkey (`self.HotKey`))
  (bind ((`Animation_24_A4CB3598496C3BC1FD4F4E93D1A8DCAF` _animation) (`Stage_18_B74872704392C835D0B405866CA6B20E` _stage)) (break `/Game/OpenRPG/SkillSystem/Structs/s_SkillInfo` (`self.Info`)))
  ;[0.04144 0.3233 1] 3. If so, begin the casting
  (`/Game/OpenRPG/SkillSystem/Blueprints/BPC_SkillsHandler.BeginSpellCast` (`self.SkillComponent`) self)
  (`/Engine/EditorBlueprintResources/StandardMacros.IsValid` _hotkey
    (:`Is Valid`
      (`Widget.SetIsEnabled` (`/Game/OpenRPG/HotKeyBarSystem/Widgets/WB_HotKey.Button` _hotkey) false))
    (:`Is Not Valid`
      _))
  (`/Engine/EditorBlueprintResources/StandardMacros.IsValid` _animation
    (:`Is Valid`
      (`self.PlayAnimation`
        (:`Completed`
          _)))
    (:`Is Not Valid`
      (`KismetSystemLibrary.Delay` (`.CastingTime_8_3D37CFFB46E6ED0908BC8AA4F550741F` (break `/Game/OpenRPG/SkillSystem/Structs/s_SkillStage` _stage)))))
  (`self.CastCompleted`))

(event `CastCompleted`
  (bind _hotkey (`self.HotKey`))
  (bind _hotkey_2 (`self.HotKey`))
  (bind _hotkey_3 (`self.HotKey`))
  (bind _cooldowntimeline (`self.CooldownTimeLine`))
  (bind _returnvalue (`TimelineComponent.GetPlaybackPosition` _cooldowntimeline))
  (bind _returnvalue_2 (`TimelineComponent.GetTimelineLength` _cooldowntimeline))
  (bind ((`Cooldown_10_E46851084141E975F173A1AF09810B85` _cooldown)) (break `/Game/OpenRPG/SkillSystem/Structs/s_SkillStage` (`.Stage_18_B74872704392C835D0B405866CA6B20E` (break `/Game/OpenRPG/SkillSystem/Structs/s_SkillInfo` (`self.Info`)))))
  (bind _returnvalue_3 (- _returnvalue_2 _returnvalue))
  ;[0 0.2123 1] 4. When cast is completed, cooldown starts
  (`/Game/OpenRPG/SkillSystem/Blueprints/BPC_SkillsHandler.EndSpellCast` (`self.SkillComponent`) self)
  (set `self.OnCooldown?` true)
  (`KismetSystemLibrary.PrintString` "Spell on CD" true true (struct :`R` 1.0 :`G` 0.064177 :`A` 1.0) 4.0)
  (`/Engine/EditorBlueprintResources/StandardMacros.IsValid` (`self.HotKey`)
    (:`Is Valid`
      (`Widget.SetIsEnabled` (`/Game/OpenRPG/HotKeyBarSystem/Widgets/WB_HotKey.Button` _hotkey_2) false)
      (`Image.SetColorAndOpacity` (`/Game/OpenRPG/HotKeyBarSystem/Widgets/WB_HotKey.Icon` _hotkey_2) (struct :`R` 0.192708 :`G` 0.192708 :`B` 0.192708 :`A` 1.0))
      (`MaterialInstanceDynamic.SetScalarParameterValue` (`/Game/OpenRPG/HotKeyBarSystem/Widgets/WB_HotKey.CooldownMaterial` _hotkey_2) "Percent" 1.0)
      (`TextBlock.SetText` (`/Game/OpenRPG/HotKeyBarSystem/Widgets/WB_HotKey.CooldownText` _hotkey_3) (`KismetTextLibrary.Conv_DoubleToText` _cooldown "HalfToEven" false false 1 324 0 0))
      (`Widget.SetVisibility` (`/Game/OpenRPG/HotKeyBarSystem/Widgets/WB_HotKey.CooldownImage` _hotkey_3) "HitTestInvisible")
      (`Widget.SetVisibility` (`/Game/OpenRPG/HotKeyBarSystem/Widgets/WB_HotKey.CooldownText` _hotkey_3) "HitTestInvisible"))
    (:`Is Not Valid`
      _))
  (`TimelineComponent.SetTimelineLength` (`self.CooldownTimeLine`) _cooldown)
  (`Timeline|CooldownTimeLine` :!via `PlayFromStart`
    (:`Update`
      (`/Engine/EditorBlueprintResources/StandardMacros.IsValid` _hotkey
        (:`Is Valid`
          (`MaterialInstanceDynamic.SetScalarParameterValue` (`/Game/OpenRPG/HotKeyBarSystem/Widgets/WB_HotKey.CooldownMaterial` _hotkey) "Percent" (- 1.0 (/ _returnvalue _returnvalue_2)))
          (`TextBlock.SetText` (`/Game/OpenRPG/HotKeyBarSystem/Widgets/WB_HotKey.CooldownText` (`self.HotKey`)) (`KismetTextLibrary.Conv_DoubleToText` _returnvalue_3 "HalfToEven" false false 1 324 0 (`KismetMathLibrary.SelectInt` 0 1 (> _returnvalue_3 1.0)))))))
    (:`Finished`
      (`self.OnCooldownExpired`))))

(event `OnCooldownExpired`
  (bind _hotkey (`self.HotKey`))
  (bind _hotkey_2 (`self.HotKey`))
  ;[0.05522 0.02144 1] 5. When cooldown finishes
  (set `self.OnCooldown?` false)
  (`/Engine/EditorBlueprintResources/StandardMacros.IsValid` _hotkey
    (:`Is Valid`
      (if (not (`/Game/OpenRPG/HotKeyBarSystem/Widgets/WB_HotKey.Deactivated?` _hotkey))
        (`Widget.SetIsEnabled` (`/Game/OpenRPG/HotKeyBarSystem/Widgets/WB_HotKey.Button` _hotkey_2) true)
        (`Image.SetColorAndOpacity` (`/Game/OpenRPG/HotKeyBarSystem/Widgets/WB_HotKey.Icon` _hotkey_2) (struct :`R` 1.0 :`G` 1.0 :`B` 1.0 :`A` 1.0)))
      (`Widget.SetVisibility` (`/Game/OpenRPG/HotKeyBarSystem/Widgets/WB_HotKey.CooldownImage` (`self.HotKey`)) "Hidden")
      (`Widget.SetVisibility` (`/Game/OpenRPG/HotKeyBarSystem/Widgets/WB_HotKey.CooldownText` (`self.HotKey`)) "Hidden"))))

(fn `UserConstructionScript`)