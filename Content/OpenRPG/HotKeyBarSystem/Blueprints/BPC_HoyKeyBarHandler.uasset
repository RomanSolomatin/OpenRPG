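; Hotkey bar component on the player controller that builds key-bound widgets and uses the inventory items linked to them.
; Each hotkey stores an inventory slot index, which follows item swaps and persists through a SaveGame object.
; Key presses use the item via the inventory handler.
; For a last-in-stack item or one specific item type, the hotkey first rebinds to another slot holding the same class, if found.
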(fn `HandleItemSwap`
  (params (`Index 1` :type Integer) (`Index 2` :type Integer))
  (locals (LocalIndex1 :type Integer) (LocalIndex2 :type Integer))
  (set `local.LocalIndex1` `Index 1`)
  (set `local.LocalIndex2` `Index 2`)
  (if (`self.Enabled?`)
    (for _array_element (`self.HotKeys`)
      (bind _inventoryindex (`/Game/OpenRPG/HotKeyBarSystem/Widgets/WB_HotKey.InventoryIndex` _array_element))
      (if (== (`local.LocalIndex1`) _inventoryindex)
        (set `/Game/OpenRPG/HotKeyBarSystem/Widgets/WB_HotKey.InventoryIndex` (`local.LocalIndex2`) _array_element)
        (elif (== _inventoryindex (`local.LocalIndex2`))
          (set `/Game/OpenRPG/HotKeyBarSystem/Widgets/WB_HotKey.InventoryIndex` (`local.LocalIndex1`) _array_element)))))
  (return))

(fn `HandleKeyPressed`
  (params (Key :type "Key Structure"))
  (locals (LocalKey :type "Key Structure"))
  (set `local.LocalKey` Key)
  (if (`self.Enabled?`)
    (if (`KismetArrayLibrary.Array_Contains` (`self.Keys`) (`local.LocalKey`))
      (for _array_element (`self.HotKeys`)
        (if (== (`/Game/OpenRPG/HotKeyBarSystem/Widgets/WB_HotKey.Key` _array_element) (`local.LocalKey`))
          (`self.UseHotKey` _array_element)
          (break)))
      (return)
      (else
        (return)))
    (else
      (return))))

(fn `Initialize`
  (params (HotKeyBarWidget :type "/Game/OpenRPG/HotKeyBarSystem/Widgets/WB_HotKeyBar Object Reference"))
  (if (`self.Enabled?`)
    (bind _output_get (set `self.HotKeyBarWidget` HotKeyBarWidget))
    (`PanelWidget.ClearChildren` (`/Game/OpenRPG/HotKeyBarSystem/Widgets/WB_HotKeyBar.HotKeyBox` _output_get))
    (`KismetArrayLibrary.Array_Clear` (`self.HotKeys`))
    (bind _asbp_custom_player_controller (cast `/Game/OpenRPG/Shared/Blueprints/BP_CustomPlayerController` (`self.GetOwner`)))
    (set `self.PlayerController` _asbp_custom_player_controller)
    (for _array_element (`self.Keys`)
      (bind _returnvalue (`|CreateWidget` "/Game/OpenRPG/HotKeyBarSystem/Widgets/WB_HotKey.WB_HotKey_C" null _array_element self))
      (`KismetArrayLibrary.Array_Add` (`self.HotKeys`) _returnvalue)
      (bind _returnvalue_2 (`HorizontalBox.AddChildToHorizontalBox` (`/Game/OpenRPG/HotKeyBarSystem/Widgets/WB_HotKeyBar.HotKeyBox` (`self.HotKeyBarWidget`)) _returnvalue))
      (`/Game/OpenRPG/HotKeyBarSystem/Widgets/WB_HotKey.Update` _returnvalue)
      (`/Game/OpenRPG/HotKeyBarSystem/Widgets/WB_HotKey.UpdateKeyText` _returnvalue)
      (`HorizontalBoxSlot.SetPadding` _returnvalue_2 (make `Margin` 0.0 0.0 (`self.PaddingBetweenHotKeys`))))
    (`self.LoadHotKeys`)
    (return)
    (else
      (return))))

(fn `ItemAlreadyInAnotherHotKey?`
  (params (ItemClass :type "/Game/OpenRPG/InventorySystem/Blueprints/Items/MasterClasses/BP_BaseItem Class Reference"))
  (returns (`Exists?` :type Boolean))
  (locals (LocalClass :type "/Game/OpenRPG/InventorySystem/Blueprints/Items/MasterClasses/BP_BaseItem Class Reference") (LocalBool :type Boolean))
  (set `local.LocalClass` ItemClass)
  (for _array_element (`self.HotKeys`)
    (if (== (`.Class_47_1920DEDC49E9F940C8E7B5830EF818FF` (break `/Game/OpenRPG/InventorySystem/Structs/s_ItemInfo` (`/Game/OpenRPG/InventorySystem/Blueprints/BPC_InventoryHandler.GetItemAtIndex` (`/Game/OpenRPG/Shared/Blueprints/BP_CustomPlayerController.BPC_InventoryHandler` (`self.PlayerController`)) (`/Game/OpenRPG/HotKeyBarSystem/Widgets/WB_HotKey.InventoryIndex` _array_element)))) (`local.LocalClass`))
      (set `local.LocalBool` true)
      (break)))
  (return (`local.LocalBool`)))

(fn `LoadHotKeys`
  (bind _returnvalue (`GameplayStatics.DoesSaveGameExist` (`self.HotKeyBarSave`)))
  (if _returnvalue
    (`/Engine/EditorBlueprintResources/StandardMacros.IsValid` (`self.HotKeyBarSaveObject`)
      (:`Is Valid`
        _)
      (:`Is Not Valid`
        (bind _returnvalue_2 (`GameplayStatics.LoadGameFromSlot` (`self.HotKeyBarSave`)))
        (bind _ashot_key_bar_save (cast `/Game/OpenRPG/HotKeyBarSystem/Blueprints/HotKeyBarSave` _returnvalue_2)
          (:`then`
            (set `self.HotKeyBarSaveObject` _ashot_key_bar_save))
          (:`CastFailed`
            (return)))))
    (for (_array_element _array_index) (`self.HotKeys`)
      (set `/Game/OpenRPG/HotKeyBarSystem/Widgets/WB_HotKey.InventoryIndex` (`|GetArrayItem` (`/Game/OpenRPG/HotKeyBarSystem/Blueprints/HotKeyBarSave.InventorySlots` (`self.HotKeyBarSaveObject`)) _array_index) _array_element)
      (`/Game/OpenRPG/HotKeyBarSystem/Widgets/WB_HotKey.Update` _array_element))
    (return)
    (else
      (return))))

(fn `SaveHotKeys`
  (bind _inventoryslots (`/Game/OpenRPG/HotKeyBarSystem/Blueprints/HotKeyBarSave.InventorySlots` (`self.HotKeyBarSaveObject`)))
  (if (`self.Enabled?`)
    (`/Engine/EditorBlueprintResources/StandardMacros.IsValid` (`self.HotKeyBarSaveObject`)
      (:`Is Valid`
        _)
      (:`Is Not Valid`
        (bind _returnvalue (`GameplayStatics.CreateSaveGameObject` "/Game/OpenRPG/HotKeyBarSystem/Blueprints/HotKeyBarSave.HotKeyBarSave_C"))
        (set `self.HotKeyBarSaveObject` _returnvalue)))
    (`KismetArrayLibrary.Array_Clear` _inventoryslots)
    (`KismetArrayLibrary.Array_Resize` _inventoryslots (`KismetArrayLibrary.Array_Length` (`self.HotKeys`)))
    (for (_array_element _array_index) (`self.HotKeys`)
      (`KismetArrayLibrary.Array_Insert` (`/Game/OpenRPG/HotKeyBarSystem/Blueprints/HotKeyBarSave.InventorySlots` (`self.HotKeyBarSaveObject`)) (`/Game/OpenRPG/HotKeyBarSystem/Widgets/WB_HotKey.InventoryIndex` _array_element) _array_index))
    (`GameplayStatics.SaveGameToSlot` (`self.HotKeyBarSaveObject`) (`self.HotKeyBarSave`))
    (return)
    (else
      (return))))

(fn `SetNewItem`
  (params (InventoryIndex :type Integer))
  (returns (NewInventoryIndex :type Integer))
  (locals (LocalIndex :type Integer))
  (bind _localindex (`local.LocalIndex`))
  (bind _bpc_inventoryhandler (`/Game/OpenRPG/Shared/Blueprints/BP_CustomPlayerController.BPC_InventoryHandler` (`self.PlayerController`)))
  (bind ((`Class_47_1920DEDC49E9F940C8E7B5830EF818FF` _class) (`Type_13_957CA2D1456D6C9D4618728B02356F59` _type)) (break `/Game/OpenRPG/InventorySystem/Structs/s_ItemInfo` (`/Game/OpenRPG/InventorySystem/Blueprints/BPC_InventoryHandler.GetItemAtIndex` _bpc_inventoryhandler _localindex)))
  (set `local.LocalIndex` InventoryIndex)
  (if (or (== (`/Game/OpenRPG/InventorySystem/Blueprints/BPC_InventoryHandler.GetAmountAtIndex` _bpc_inventoryhandler _localindex) 1) (`|EnumEquality` _type "NewEnumerator4"))
    (return (`/Game/OpenRPG/InventorySystem/Blueprints/BPC_InventoryHandler.GetSlotWithSameItem` (`/Game/OpenRPG/Shared/Blueprints/BP_CustomPlayerController.BPC_InventoryHandler` (`self.PlayerController`)) _class (`local.LocalIndex`)))
    (else
      (return -1))))

(fn `UpdateHotKey`
  (params (InventoryIndex :type Integer))
  (locals (LocalIndex :type Integer))
  (set `local.LocalIndex` InventoryIndex)
  (if (`self.Enabled?`)
    (for _array_element (`self.HotKeys`)
      (if (== (`/Game/OpenRPG/HotKeyBarSystem/Widgets/WB_HotKey.InventoryIndex` _array_element) (`local.LocalIndex`))
        (`/Game/OpenRPG/HotKeyBarSystem/Widgets/WB_HotKey.Update` _array_element)))
    (return)
    (else
      (return))))

(fn `UseHotKey`
  (params (HotKeyWidget :type "/Game/OpenRPG/HotKeyBarSystem/Widgets/WB_HotKey Object Reference"))
  (locals (LocalUsedHotKey :type "/Game/OpenRPG/HotKeyBarSystem/Widgets/WB_HotKey Object Reference") (LocalInventoryIndex :type Integer :default 0) (LocalFoundIndex :type Integer :default 0))
  (`/Engine/EditorBlueprintResources/StandardMacros.IsValid` HotKeyWidget
    (:`Is Valid`
      (bind _output_get (set `local.LocalUsedHotKey` HotKeyWidget))
      (set `local.LocalInventoryIndex` (`/Game/OpenRPG/HotKeyBarSystem/Widgets/WB_HotKey.InventoryIndex` _output_get))
      (bind _newinventoryindex (`self.SetNewItem` (`local.LocalInventoryIndex`)))
      (bind _output_get_2 (set `local.LocalFoundIndex` _newinventoryindex))
      (if (!= _output_get_2 -1)
        (set `/Game/OpenRPG/HotKeyBarSystem/Widgets/WB_HotKey.InventoryIndex` (`local.LocalFoundIndex`) (`local.LocalUsedHotKey`)) ; Set the new index of the hotkeybar
        (`/Game/OpenRPG/HotKeyBarSystem/Widgets/WB_HotKey.Update` (`local.LocalUsedHotKey`)))
      (`/Game/OpenRPG/InventorySystem/Blueprints/BPC_InventoryHandler.UseItemAtIndex` (`/Game/OpenRPG/Shared/Blueprints/BP_CustomPlayerController.BPC_InventoryHandler` (`self.PlayerController`)) (`local.LocalInventoryIndex`))
      (return))
    (:`Is Not Valid`
      (return))))