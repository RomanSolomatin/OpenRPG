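; BP_BaseEquipment is the master class for equippable inventory items, overriding UseItem so that using an item equips it instead of running item-specific logic.
; It calls the parent UseItem to set shared variables, then reads the item's info from the clicked slot through the player controller's inventory handler.
; The equipment handler's EquipItem receives that info and handles removal from the slot, then the item actor destroys itself.
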(event `self.UseItem`
  (params (`Clicked Slot Index` :type Integer) (PlayerController :type "/Game/OpenRPG/Shared/Blueprints/BP_CustomPlayerController Object Reference"))
  ;[0.1043 1 0.1512] Equipment items are just equipped, they dont have special logic so they dont use OnItemUsed, and we have to check some things before removing it from the inventory (handled by the EquipItem function)
  (`parent.UseItem` `Clicked Slot Index` PlayerController) ; Remember that in the BaseItem class we just set the variables, this call avoid us to set them manually again :D
  (set `self.ItemInfo` (`/Game/OpenRPG/InventorySystem/Blueprints/BPC_InventoryHandler.GetItemAtIndex` (`/Game/OpenRPG/Shared/Blueprints/BP_CustomPlayerController.BPC_InventoryHandler` (`self.PlayerController`)) (`self.ClickedSlotIndex`))) ; Load custom info from the inventory
  (`|ExecutionSequence`
    (:`then_0`
      (`/Game/OpenRPG/EquipmentSystem/Blueprints/BPC_EquipmentHandler.EquipItem` (`/Game/OpenRPG/Shared/Blueprints/BP_CustomPlayerController.BPC_EquipmentHandler` (`self.PlayerController`)) (`self.ItemInfo`) (`self.ClickedSlotIndex`)) ; This function will handle the remove from the inventory slot with the ClickedSlotIndex
    )
    (:`then_1`
      (`self.K2_DestroyActor`))))

(fn `UserConstructionScript`
  (`parent.UserConstructionScript`))