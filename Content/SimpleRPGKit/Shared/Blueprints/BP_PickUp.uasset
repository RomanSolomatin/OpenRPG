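; World item pickup for the RPG kit's demo, showing a name, amount and interact prompt.
; Construction loads ItemInfo from DT_Items by ItemID to set mesh and interact radius; an ID of -1 uses the existing ItemInfo at BeginPlay.
; Table-based items roll equipment attributes valued -1 within min/max at BeginPlay.
; Sphere overlap registers it in the character's NearbyItems and toggles the text; OnPickUp adds it to inventory, destroying it on success.
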(event `self.ReceiveBeginPlay`
  ;[0.9062 0.3879 0.2239] Remember that this is just a demo to test the system
  (bind _aswb_interact_text (cast `/Game/SimpleRPGKit/Shared/Widgets/WB_InteractText` (`WidgetComponent.GetUserWidgetObject` (`self.Text`))))
  (`/Game/SimpleRPGKit/Shared/Widgets/WB_InteractText.Initialize` _aswb_interact_text (`|FormatText` "{Name} x{Amount}" (`KismetTextLibrary.Conv_NameToText` (`.Name_48_5152AB7A4A14C21B2A5660A506525218` (break `/Game/SimpleRPGKit/InventorySystem/Structs/s_ItemInfo` (`self.ItemInfo`)))) (`self.Amount`)) "Press [E] to interact!")
  (if (!= (`self.ItemID`) -1)
    (`self.RandomizeEquipmentAttributes`)
    (else
      (`self.SetVisualProperties`))))

(event `OnPickUp`
  (params (PlayerController :type "/Game/SimpleRPGKit/Shared/Blueprints/BP_CustomPlayerController Object Reference"))
  ;[0.9062 0.3879 0.2239] Remember that this is just a demo to test the system
  (bind _output_get (set `self.PlayerController` PlayerController))
  (bind _success_ (`/Game/SimpleRPGKit/InventorySystem/Blueprints/BPC_InventoryHandler.AddIItem (Public)` (`/Game/SimpleRPGKit/Shared/Blueprints/BP_CustomPlayerController.BPC_InventoryHandler` _output_get) (`self.ItemInfo`) (`self.Amount`))) ; Use the reference of the already spawned item
  (if _success_
    (`KismetArrayLibrary.Array_RemoveItem` (`/Game/SimpleRPGKit/Shared/Blueprints/BP_MasterCharacter.NearbyItems` (`/Game/SimpleRPGKit/Shared/Blueprints/BP_CustomPlayerController.ControlledPawn` (`self.PlayerController`))) self) ; Updates the nearby items in the player controller
    (`self.K2_DestroyActor`) ; Destroy self
    (else
      (`KismetSystemLibrary.PrintString` "Error while adding item to inventory"))))

(event `self.Colision.OnComponentBeginOverlap`
  (params (OverlappedComponent :type "PrimitiveComponent Object Reference") (OtherActor :type "Actor Object Reference") (OtherComp :type "PrimitiveComponent Object Reference") (OtherBodyIndex :type Integer) (bFromSweep :type Boolean) (SweepResult :type "HitResult Structure (by ref)"))
  ;[0.9062 0.3879 0.2239] Remember that this is just a demo to test the system
  (bind _asbp_master_character (cast `/Game/SimpleRPGKit/Shared/Blueprints/BP_MasterCharacter` OtherActor))
  (`KismetArrayLibrary.Array_Add` (`/Game/SimpleRPGKit/Shared/Blueprints/BP_MasterCharacter.NearbyItems` _asbp_master_character) self)
  (`SceneComponent.SetVisibility` (`self.Text`) true false))

(event `self.Colision.OnComponentEndOverlap`
  (params (OverlappedComponent :type "PrimitiveComponent Object Reference") (OtherActor :type "Actor Object Reference") (OtherComp :type "PrimitiveComponent Object Reference") (OtherBodyIndex :type Integer))
  ;[0.9062 0.3879 0.2239] Remember that this is just a demo to test the system
  (bind _asbp_master_character (cast `/Game/SimpleRPGKit/Shared/Blueprints/BP_MasterCharacter` OtherActor))
  (`KismetArrayLibrary.Array_RemoveItem` (`/Game/SimpleRPGKit/Shared/Blueprints/BP_MasterCharacter.NearbyItems` _asbp_master_character) self)
  (`SceneComponent.SetVisibility` (`self.Text`) false false))

(fn `RandomizeEquipmentAttributes`
  (for (_array_element _array_index) (`.Attributes_18_773B08524147154330A5BCA36C2A6DB1` (break `/Game/SimpleRPGKit/EquipmentSystem/Structs/s_EquipmentInfo` (`.EquipmentInfo_51_8C46272242ED9B623F8E07929B5947B1` (break `/Game/SimpleRPGKit/InventorySystem/Structs/s_ItemInfo` (`self.ItemInfo`)))))
    (bind (_attributetype _minvalue _maxvalue _value) (break `/Game/SimpleRPGKit/EquipmentSystem/Structs/s_Attribute` _array_element))
    (`KismetArrayLibrary.Array_Set` (`.Attributes_18_773B08524147154330A5BCA36C2A6DB1` (break `/Game/SimpleRPGKit/EquipmentSystem/Structs/s_EquipmentInfo` (`.EquipmentInfo_51_8C46272242ED9B623F8E07929B5947B1` (break `/Game/SimpleRPGKit/InventorySystem/Structs/s_ItemInfo` (`self.ItemInfo`))))) _array_index (make `/Game/SimpleRPGKit/EquipmentSystem/Structs/s_Attribute` _attributetype _minvalue _maxvalue (`KismetMathLibrary.SelectInt` _value (`KismetMathLibrary.RandomIntegerInRange` _minvalue _maxvalue) (!= _value -1)))))
  (return))

(fn `SetVisualProperties`
  (bind ((`MeshScale_36_871784B64E173F2DA276F092C5765EA8` _meshscale) (`InteractRadius_39_72B75A514A28C5CCF441DFB1ABD825FC` _interactradius)) (break `/Game/SimpleRPGKit/InventorySystem/Structs/s_ItemInfo` (`self.ItemInfo`)))
  (bind ((`Mesh_33_8E32AF884495DEACF333A795383B8E4A` _mesh)) (break `/Game/SimpleRPGKit/InventorySystem/Structs/s_ItemInfo` (`self.ItemInfo`)))
  (`StaticMeshComponent.SetStaticMesh` (`self.DefaultMesh`) _mesh)
  (`PrimitiveComponent.SetMaterial` (`self.DefaultMesh`) 0 (`StaticMesh.GetMaterial` _mesh 0))
  (`SceneComponent.SetWorldScale3D` (`self.DefaultMesh`) _meshscale)
  (`SphereComponent.SetSphereRadius` (`self.Colision`) _interactradius false)
  (return))

(fn `UserConstructionScript`
  (if (!= (`self.ItemID`) -1)
    (bind _returnvalue (`|GetDataTableRow` "/Game/SimpleRPGKit/InventorySystem/Blueprints/Items/DT_Items.DT_Items" (`KismetStringLibrary.Conv_StringToName` (`KismetStringLibrary.Conv_IntToString` (`self.ItemID`)))) ; Get the info from the data table
      (:`then`
        (bind _output_get (set `self.ItemInfo` _returnvalue))
        (if (`KismetSystemLibrary.IsValidClass` (`.Class_47_1920DEDC49E9F940C8E7B5830EF818FF` (break `/Game/SimpleRPGKit/InventorySystem/Structs/s_ItemInfo` _output_get)))
          (`self.SetVisualProperties`))))))